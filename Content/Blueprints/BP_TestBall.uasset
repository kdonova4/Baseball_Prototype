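; Ball actor for a home run derby that faces the player's BallDirection on spawn and scores where it lands.
; Tick scales Sphere with camera distance and predicts Sphere1's projectile path, though the landing-marker logic using it is disconnected.
; Sphere1's first overlap adds a home run on HomerunDetect, otherwise an out if GotHit, updating the player's derby UI.
; After a short delay it clears GotHit and destroys itself.
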(event OnComponentHit(Sphere1)
  (params (HitComponent :type Primitive%20Component%20Object%20Reference) (OtherActor :type Actor%20Object%20Reference) (OtherComp :type Primitive%20Component%20Object%20Reference) (NormalImpulse :type Vector :default "0, 0, 0") (Hit :type Hit%20Result%20Structure%20%28by%20ref%29)))

(event OnComponentHit(Sphere)
  (params (HitComponent :type Primitive%20Component%20Object%20Reference) (OtherActor :type Actor%20Object%20Reference) (OtherComp :type Primitive%20Component%20Object%20Reference) (NormalImpulse :type Vector :default "0, 0, 0") (Hit :type Hit%20Result%20Structure%20%28by%20ref%29)))

(event OnComponentBeginOverlap(Sphere1)
  (params (OverlappedComponent :type Primitive%20Component%20Object%20Reference) (OtherActor :type Actor%20Object%20Reference) (OtherComp :type Primitive%20Component%20Object%20Reference) (OtherBodyIndex :type Integer) (bFromSweep :type Boolean) (SweepResult :type Hit%20Result%20Structure%20%28by%20ref%29))
  (bind _returnvalue (Utilities|GetObjectName OtherActor))
  (bind _tpc (Variables|Default|GetTPC))
  (bind _tpc_2 (Variables|Default|GetTPC))
  (if (not (Variables|Default|Getlanded))
    (Variables|Default|Setlanded true)
    (Development|PrintString _returnvalue false false)
    (if (Utilities|Enum|Equal(Enum) _returnvalue "HomerunDetect")
      (bind _result (Math|Integer|IncrementInt (Variables|/Game/ThirdPersonBP/Blueprints/ThirdPersonCharacter.ThirdPersonCharacter_C|GetHomeruns _tpc))
        (:%20%20
          (Default|IncreaseHomeruns (Variables|/Game/ThirdPersonBP/Blueprints/ThirdPersonCharacter.ThirdPersonCharacter_C|GetHome_Run_DerbyUI _tpc) _result)))
      (elif (Variables|/Game/ThirdPersonBP/Blueprints/ThirdPersonCharacter.ThirdPersonCharacter_C|GetGotHit _tpc_2)
        (bind _result_2 (Math|Integer|IncrementInt (Variables|/Game/ThirdPersonBP/Blueprints/ThirdPersonCharacter.ThirdPersonCharacter_C|GetOuts _tpc_2))
          (:%20%20
            (bind _output_get (Variables|/Game/ThirdPersonBP/Blueprints/ThirdPersonCharacter.ThirdPersonCharacter_C|SetOuts _tpc_2 _result_2))
            (Default|IncreaseOuts (Variables|/Game/ThirdPersonBP/Blueprints/ThirdPersonCharacter.ThirdPersonCharacter_C|GetHome_Run_DerbyUI _tpc_2) _output_get)))))
    (Utilities|FlowControl|Delay 3.0)
    (Variables|/Game/ThirdPersonBP/Blueprints/ThirdPersonCharacter.ThirdPersonCharacter_C|SetGotHit (Variables|Default|GetTPC) false)
    (Actor|DestroyActor)))

(event Custom|Predict)

(event EventBeginPlay
  (Variables|Default|SetPlayerCam (Variables|/Game/ThirdPersonBP/Blueprints/ThirdPersonCharacter.ThirdPersonCharacter_C|GetFollowCamera (.AsThird%20Person%20Character (Utilities|Casting|CastToThirdPersonCharacter (Game|GetPlayerCharacter 0)))))
  (bind _asthird_person_character (Utilities|Casting|CastToThirdPersonCharacter (Game|GetPlayerCharacter 0)))
  (bind _output_get (Variables|Default|SetTPC _asthird_person_character))
  (Transformation|SetActorRotation (Math|Rotator|FindLookatRotation (Transformation|GetActorLocation) (Variables|/Game/ThirdPersonBP/Blueprints/ThirdPersonCharacter.ThirdPersonCharacter_C|GetBallDirection _output_get))))

(event Collision|EventActorBeginOverlap
  (params (OtherActor :type Actor%20Object%20Reference)))

(event EventTick
  (params (DeltaSeconds :type Float%20%28single-precision%29))
  (bind _sphere1 (Variables|Default|GetSphere1))
  (Variables|Default|SetDistance (Math|Vector|VectorLength (- (Transformation|GetWorldLocation (Variables|Default|GetSphere)) (Transformation|GetWorldLocation (Variables|Default|GetPlayerCam)))))
  (Transformation|SetRelativeTransform (Variables|Default|GetSphere) (Math|Transform|MakeTransform "0, 0, 0" "0, 0, 0" (Math|Conversions|ToVector(Float) (Math|Float|Lerp 0.0625 2.75 (Math|Float|NormalizetoRange (/ (Variables|Default|GetDistance) (Variables|Default|GetStartScaleDistance)) 0.0 4e+02)))) false false)
  (bind _outhit (Class|GameplayStatics|BlueprintPredictProjectilePathbyObjectType (Transformation|GetWorldLocation _sphere1) (Transformation|GetComponentVelocity _sphere1) true 0.0 (Utilities|Array|MakeArray "ObjectTypeQuery1") false 0 "None" 0.0 6.0 1e+01)))

(fn ConstructionScript)

(fn PredictBallPath
  (params (Velocity :type Vector)))