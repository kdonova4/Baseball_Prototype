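; BP_Thrower is an actor built to throw projectiles, but its throwing and aiming logic is disconnected.
; Tick only caches the player as ThirdPersonCharacter.
; An unwired timeline branch would spawn BP_Projectile at ThrowPosition, apply a fixed world-space impulse and gate repeats with CanShoot and a short delay.
; Another unwired node would rotate the actor toward an offset from the player's StrikeZone center.
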(event EventTick
  (params (DeltaSeconds :type Float%20%28single-precision%29))
  (bind _asthird_person_character (Utilities|Casting|CastToThirdPersonCharacter (Game|GetPlayerCharacter 0))))

(fn ConstructionScript)