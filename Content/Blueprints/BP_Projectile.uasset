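; Pitched baseball projectile for a batting game, pushed each tick by its Pitch impulse while reporting position and speed to the player's timing logic.
; A predicted-path trace flags hits or foul tips on swings, while forward line traces classify strike or ball and record the location.
; Catcher overlap updates count and discipline score, plays the glove sound and briefly spawns a location marker.
; Striking the Hit Zone enables gravity and plays bat sound.
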(event OnComponentBeginOverlap(Sphere1)
  (params (OverlappedComponent :type Primitive%20Component%20Object%20Reference) (OtherActor :type Actor%20Object%20Reference) (OtherComp :type Primitive%20Component%20Object%20Reference) (OtherBodyIndex :type Integer) (bFromSweep :type Boolean) (SweepResult :type Hit%20Result%20Structure%20%28by%20ref%29))
  (bind _returnvalue (Utilities|GetObjectName OtherComp))
  (bind _as_third_person_character (Variables|Default|GetAs%20Third%20Person%20Character))
  (if (Utilities|Enum|Equal(Enum) _returnvalue "Catcher")
    (Development|PrintString _returnvalue)
    (if (Variables|/Game/ThirdPersonBP/Blueprints/ThirdPersonCharacter.ThirdPersonCharacter_C|Getswung? _as_third_person_character)
      _
      (else
        (Default|Looking _as_third_person_character)))
    (Development|PrintString (Utilities|String|ToString(Boolean) (Variables|Default|GetisStrike?)) true true "(R=0.101539,G=1.000000,B=0.000000,A=1.000000)")
    (CallFunction|SpawnIndicator)
    (CallFunction|CatchBall)))

(event Custom|Spawn%20Indicator
  (bind _as_third_person_character (Variables|Default|GetAs%20Third%20Person%20Character))
  (if (Variables|Default|GetisStrike?)
    (if (Variables|/Game/ThirdPersonBP/Blueprints/ThirdPersonCharacter.ThirdPersonCharacter_C|Getswung? _as_third_person_character)
      _
      (else
        (Default|DisciplineFuncSubtractScore _as_third_person_character 100)
        (Default|DisciplineFuncSubtractBalls _as_third_person_character)
        (Default|AddStrike _as_third_person_character)))
    (bind _returnvalue (Game|SpawnActorfromClass "/Game/Blueprints/Strike.Strike_C" (Variables|Default|GetBallLoc) "Undefined" 0 0))
    (Development|SetHiddeninGame (Variables|/Game/ThirdPersonBP/Blueprints/ThirdPersonCharacter.ThirdPersonCharacter_C|GetOutline (Variables|Default|GetAs%20Third%20Person%20Character)) false false)
    (Utilities|FlowControl|Delay 2.0)
    (Actor|DestroyActor _returnvalue)
    (elif (Variables|/Game/ThirdPersonBP/Blueprints/ThirdPersonCharacter.ThirdPersonCharacter_C|Getswung? _as_third_person_character)
      (Default|DisciplineFuncSubtractScore _as_third_person_character 150)
      (bind _returnvalue_2 (Game|SpawnActorfromClass "/Game/Blueprints/Strike.Strike_C" (Variables|Default|GetBallLoc) "Undefined" 0 0))
      (Development|SetHiddeninGame (Variables|/Game/ThirdPersonBP/Blueprints/ThirdPersonCharacter.ThirdPersonCharacter_C|GetOutline (Variables|Default|GetAs%20Third%20Person%20Character)) false false)
      (Utilities|FlowControl|Delay 2.0)
      (Actor|DestroyActor _returnvalue_2)
      (else
        (Default|DisciplineFuncAddScore (Variables|Default|GetAs%20Third%20Person%20Character) 100)
        (Default|AddBall _as_third_person_character)
        (bind _returnvalue_3 (Game|SpawnActorfromClass "/Game/Blueprints/Ball.Ball_C" (Variables|Default|GetBallLoc) "Undefined" 0 0))
        (Development|SetHiddeninGame (Variables|/Game/ThirdPersonBP/Blueprints/ThirdPersonCharacter.ThirdPersonCharacter_C|GetOutline (Variables|Default|GetAs%20Third%20Person%20Character)) false false)
        (Utilities|FlowControl|Delay 2.0)
        (Actor|DestroyActor _returnvalue_3)))))

(event Custom|CatchBall
  (bind _as_third_person_character (Variables|Default|GetAs%20Third%20Person%20Character))
  (if (or (Variables|/Game/ThirdPersonBP/Blueprints/ThirdPersonCharacter.ThirdPersonCharacter_C|GetGotHit _as_third_person_character) (Variables|/Game/ThirdPersonBP/Blueprints/ThirdPersonCharacter.ThirdPersonCharacter_C|GetFouledOff _as_third_person_character))
    _
    (else
      (Audio|PlaySoundatLocation (Variables|Default|GetGloveSound) (Transformation|GetWorldLocation (Variables|Default|GetSphere1)) "0, 0, 0" 1.0 1.0 0.0 0 0 0)))
  (Audio|Components|Audio|Stop (Variables|Default|GetAudio)))

(event EventBeginPlay
  (Audio|Components|Audio|Play (Variables|Default|GetAudio) 0.0)
  (bind _asthird_person_character (Utilities|Casting|CastToThirdPersonCharacter (Game|GetPlayerCharacter 0)))
  (Variables|Default|SetAs%20Third%20Person%20Character _asthird_person_character))

(event Collision|EventActorBeginOverlap
  (params (OtherActor :type Actor%20Object%20Reference)))

(event EventTick
  (params (DeltaSeconds :type Float%20%28single-precision%29))
  (bind _as_third_person_character (Variables|Default|GetAs%20Third%20Person%20Character))
  (bind _sphere1 (Variables|Default|GetSphere1))
  (bind _sphere (Variables|Default|GetSphere))
  (bind _as_third_person_character_2 (Variables|Default|GetAs%20Third%20Person%20Character))
  (bind _sphere1_2 (Variables|Default|GetSphere1))
  (bind _returnvalue (Math|Vector|GetForwardVector _sphere))
  (bind _returnvalue_2 (Transformation|GetWorldLocation _sphere))
  (bind _swung_ (Variables|/Game/ThirdPersonBP/Blueprints/ThirdPersonCharacter.ThirdPersonCharacter_C|Getswung? _as_third_person_character))
  (bind _returnvalue_3 (* _returnvalue 65.0))
  (bind _returnvalue_4 (+ _returnvalue_2 _returnvalue_3))
  (if (Variables|/Game/ThirdPersonBP/Blueprints/ThirdPersonCharacter.ThirdPersonCharacter_C|GetGotHit _as_third_person_character_2)
    (Audio|Components|Audio|Stop (Variables|Default|GetAudio)))
  (Default|Timing _as_third_person_character_2 (Variables|/Game/ThirdPersonBP/Blueprints/ThirdPersonCharacter.ThirdPersonCharacter_C|Getcalculate _as_third_person_character_2) (Transformation|GetWorldLocation _sphere1_2) (.x (Transformation|GetComponentVelocity _sphere1_2)))
  ;[1 1 1] use for location clue in zone pitching not for stike confirmation
  (if (Variables|Default|GetHIT)
    _
    (else
      _))
  (Utilities|Casting|CastToThirdPersonCharacter (Game|GetPlayerCharacter 0))
  (Utilities|FlowControl|Delay 0.01)
  (Physics|AddImpulse (Variables|Default|GetSphere1) (* (Variables|Default|GetPitch) (Utilities|Time|GetWorldDeltaSeconds)) "None" true)
  (bind _outhit (Class|GameplayStatics|BlueprintPredictProjectilePathbyTraceChannel (Transformation|GetWorldLocation _sphere1) (Transformation|GetComponentVelocity _sphere1) true 0.0 "ECC_Destructible" true 0 "None" 0.0 15.0 1.0 1.0))
  (if (and _swung_ (Utilities|Enum|Equal(Enum) (Utilities|GetObjectName (.hitcomponent _outhit)) "Hit Zone"))
    (Variables|/Game/ThirdPersonBP/Blueprints/ThirdPersonCharacter.ThirdPersonCharacter_C|SetHit? _as_third_person_character true)
    (Variables|/Game/ThirdPersonBP/Blueprints/ThirdPersonCharacter.ThirdPersonCharacter_C|SetNormalZ (Variables|Default|GetAs%20Third%20Person%20Character) (.z (.normal _outhit)))
    (elif (and _swung_ (Utilities|Enum|Equal(Enum) (Utilities|GetObjectName (.hitcomponent _outhit)) "Foul Zone"))
      (Variables|/Game/ThirdPersonBP/Blueprints/ThirdPersonCharacter.ThirdPersonCharacter_C|SetFoulTip? _as_third_person_character true)))
  (bind _outhit_2 (Collision|LineTraceForObjects _returnvalue_2 _returnvalue_4 (Utilities|Array|MakeArray "ObjectTypeQuery5") false 0 "None"))
  (if (Utilities|Enum|Equal(Enum) (Utilities|GetObjectName (.hitcomponent _outhit_2)) "Hit Zone")
    _
    (else
      _))
  (bind (_outhit_3 _returnvalue_5) (Collision|LineTraceForObjects _returnvalue_2 _returnvalue_4 (Utilities|Array|MakeArray "ObjectTypeQuery6") false 0 "None"))
  (if (and (Utilities|Enum|Equal(Enum) (Utilities|GetObjectName (.hitcomponent _outhit_3)) "Strike Zone") _returnvalue_5)
    (Variables|Default|SetisStrike? true)
    (if (and (Variables|Default|GetStrike) (not (Variables|Default|GetSpawned)))
      (Variables|Default|SetBallLoc (Math|Conversions|ToTransform(Vector) (Utilities|Array|Get(acopy) (Utilities|Array|MakeArray (.impactpoint _outhit_3)) (Utilities|Array|LastIndex (Utilities|Array|MakeArray (.impactpoint _outhit_3)))))))
    (elif (Utilities|Array|ContainsItem (Utilities|Array|MakeArray (Utilities|String|ToString(Text) (Utilities|Text|ToText(String) "Ball Zone")) (Utilities|String|ToString(Text) (Utilities|Text|ToText(String) "Ball Zone1")) (Utilities|String|ToString(Text) (Utilities|Text|ToText(String) "Ball Zone2")) (Utilities|String|ToString(Text) (Utilities|Text|ToText(String) "Ball Zone3"))) (Utilities|GetObjectName (.hitcomponent _outhit_3)))
      (Variables|Default|SetisBall? false)
      (if (and (Variables|Default|GetBall) (not (Variables|Default|GetSpawned)))
        (Variables|Default|SetBallLoc (Math|Conversions|ToTransform(Vector) (Utilities|Array|Get(acopy) (Utilities|Array|MakeArray (.impactpoint _outhit_3)) (Utilities|Array|LastIndex (Utilities|Array|MakeArray (.impactpoint _outhit_3)))))))
      (else
        (Utilities|FlowControl|Delay 3.0)
        (Actor|DestroyActor)))))

(event Collision|EventHit
  (params (MyComp :type Primitive%20Component%20Object%20Reference) (Other :type Actor%20Object%20Reference) (OtherComp :type Primitive%20Component%20Object%20Reference) (bSelfMoved :type Boolean) (HitLocation :type Vector :default "0, 0, 0") (HitNormal :type Vector :default "0, 0, 0") (NormalImpulse :type Vector :default "0, 0, 0") (Hit :type Hit%20Result%20Structure%20%28by%20ref%29))
  (if (Utilities|Enum|Equal(Enum) (Utilities|GetObjectName OtherComp) "Hit Zone")
    (Development|PrintString "Hello" true true "(R=0.000000,G=0.660000,B=1.000000,A=1.000000)" 1.0)
    (Physics|SetEnableGravity (Variables|Default|GetSphere1) true)
    (Variables|Default|SetHIT true)
    (Audio|SpawnSoundatLocation "/Game/bat+hit+ball.bat+hit+ball" (Transformation|GetWorldLocation (Variables|Default|GetSphere1)) "0, 0, 0" 1.0 1.0 0.0 0 0)))

(fn ConstructionScript)